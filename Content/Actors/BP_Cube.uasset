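; BP_Cube is a roaming cube that gets painted with the player material and spreads that paint to other cubes.
; A looping timer with a randomized start applies random horizontal velocity-change impulses, keeping movement frame-rate independent.
; Each cube increments BP_Character's DefaultCubeAmount on spawn.
; Overlaps with the character or a painted cube paint it, decrement that count and spawn particles, with sound only for cube-to-cube painting.
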(event Custom|Move
  ;[1 1 1] Рух (не залежить від частоти кадрів)
  (Physics|AddImpulse (Variables|Default|GetStaticMesh) (Math|Vector|MakeVector (Math|Random|RandomFloatinRange -4e+02 4e+02) (Math|Random|RandomFloatinRange -4e+02 4e+02) 0.0) "None" true))

(event Collision|EventActorBeginOverlap
  (params (OtherActor :type Actor%20Object%20Reference))
  ;[1 1 1] Фарбування
  (bind _asbp_character (Utilities|Casting|CastToBP_Character OtherActor)
    (:then
      (if (!= (Rendering|Material|GetMaterial (Variables|Default|GetStaticMesh) 0) "/Game/Materials/PlayerMaterial.PlayerMaterial")
        (Rendering|Material|SetMaterial (Variables|Default|GetStaticMesh) 0 "/Game/Materials/PlayerMaterial.PlayerMaterial")
        (bind _result (Math|Integer|DecrementInt (Variables|/Game/Actors/BP_Character.BP_Character_C|GetDefaultCubeAmount _asbp_character))
          (:%20%20
            (Variables|/Game/Actors/BP_Character.BP_Character_C|SetDefaultCubeAmount _asbp_character _result)
            ;[1 1 1] Ефект частинок при фарбуванні
            (Effects|SpawnEmitteratLocation "/Game/ParticleSystem/PS_HitRed.PS_HitRed" (Transformation|GetActorLocation) :!label _label)))))
    (:CastFailed
      (bind _asbp_cube (Utilities|Casting|CastToBP_Cube OtherActor))
      (if (== "/Game/Materials/PlayerMaterial.PlayerMaterial" (Rendering|Material|GetMaterial (Variables|Default|GetStaticMesh) 0))
        (if (!= "/Game/Materials/PlayerMaterial.PlayerMaterial" (Rendering|Material|GetMaterial (Variables|BP_Cube_C|GetStaticMesh _asbp_cube) 0))
          (Rendering|Material|SetMaterial (Variables|BP_Cube_C|GetStaticMesh _asbp_cube) 0 "/Game/Materials/PlayerMaterial.PlayerMaterial")
          (bind _outactors (Actor|GetAllActorsOfClass "/Game/Actors/BP_Character.BP_Character_C"))
          (bind _result_2 (Math|Integer|DecrementInt (Variables|/Game/Actors/BP_Character.BP_Character_C|GetDefaultCubeAmount (Utilities|Array|Get(acopy) _outactors)))
            (:%20%20
              (Variables|/Game/Actors/BP_Character.BP_Character_C|SetDefaultCubeAmount (Utilities|Array|Get(acopy) _outactors) _result_2)
              ;[1 1 1] Звук фарбування
              (Audio|PlaySoundatLocation "/Game/Audio/clap_Cue.clap_Cue" (Transformation|GetActorLocation) "0, 0, 0" 1.0 1.0 0.0 0 0 0 0)
              (goto _label))))))))

(event EventBeginPlay
  ;[1 1 1] Підрахунок кількості кубів на сцені
  (Utilities|Time|SetTimerbyEvent (delegate Custom|Move) 0.2 true 0.1 1.0)
  (bind _outactors (Actor|GetAllActorsOfClass "/Game/Actors/BP_Character.BP_Character_C"))
  (bind _result (Math|Integer|IncrementInt (Variables|/Game/Actors/BP_Character.BP_Character_C|GetDefaultCubeAmount (Utilities|Array|Get(acopy) _outactors)))
    (:%20%20
      (Variables|/Game/Actors/BP_Character.BP_Character_C|SetDefaultCubeAmount (Utilities|Array|Get(acopy) _outactors) _result))))

(fn ConstructionScript)