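; Player-controlled physics ball that shows the HUD on start and declares victory when its cube count reaches zero.
; Movement axes push the Sphere along the Camera's forward and right vectors with velocity-change impulses scaled by Speed and delta time, while look axes drive controller yaw and pitch.
; Tick polls DefaultCubeAmount, using a Once flag to show the victory widget and sound a single time.
; Every actor overlap plays a clap sound.
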(event EventTick
  (params (DeltaSeconds :type Float%20%28single-precision%29))
  ;[1 1 1] Перемога
  (if (and (== (Variables|Default|GetDefaultCubeAmount) 0) (Variables|Default|GetOnce))
    (bind _returnvalue (UserInterface|CreateWidget "/Game/UI/WBP_Victory.WBP_Victory_C"))
    (UserInterface|Viewport|AddtoViewport _returnvalue 0)
    (Audio|PlaySoundatLocation "/Game/Audio/Victory.Victory" (Transformation|GetActorLocation) "0, 0, 0" 1.0 1.0 0.0 0 0 0 0)
    (Variables|Default|SetOnce false)))

(event EventBeginPlay
  ;[1 1 1] Інтерфейс
  (bind _returnvalue (UserInterface|CreateWidget "/Game/UI/WBP_HUD.WBP_HUD_C"))
  (UserInterface|Viewport|AddtoViewport _returnvalue 0))

(event Collision|EventActorBeginOverlap
  (params (OtherActor :type Actor%20Object%20Reference))
  ;[1 1 1] Звук при зіткненні персонажа
  (Audio|PlaySoundatLocation "/Game/Audio/clap_Cue.clap_Cue" (Transformation|GetActorLocation) "0, 0, 0" 1.0 1.0 0.0 0 0 0 0))

(event Input|AxisEvents|InputAxisForwardBack
  (params (AxisValue :type Float%20%28single-precision%29))
  ;[1 1 1] Рух сфери (не залежить від частоти кадрів)
  (Physics|AddImpulse (Variables|Default|GetSphere) (* (Math|Vector|GetForwardVector (Variables|Default|GetCamera)) (* AxisValue (Variables|Default|GetSpeed)) (stale EventTick DeltaSeconds)) "None" true))

(event Input|AxisEvents|InputAxisRightLeft
  (params (AxisValue :type Float%20%28single-precision%29))
  ;[1 1 1] Рух сфери (не залежить від частоти кадрів)
  (Physics|AddImpulse (Variables|Default|GetSphere) (* (* (Variables|Default|GetSpeed) AxisValue) (Math|Vector|GetRightVector (Variables|Default|GetCamera)) (stale EventTick DeltaSeconds)) "None" true))

(event Input|AxisEvents|InputAxisLookUp
  (params (AxisValue :type Float%20%28single-precision%29))
  ;[1 1 1] Контроль камери
  (Pawn|Input|AddControllerPitchInput AxisValue))

(event Input|AxisEvents|InputAxisLookRight
  (params (AxisValue :type Float%20%28single-precision%29))
  ;[1 1 1] Контроль камери
  (Pawn|Input|AddControllerYawInput AxisValue))

(fn ConstructionScript)